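; Player-controllable tank Blueprint that handles driving, camera orbit and firing.
; BeginPlay hands the barrel and turret to TankAiming and both tracks to TankMovement.
; Input axes rotate the azimuth gimbal and spring arm, scaled by delta time, or pass move and turn intent to TankMovement; the Fire action calls Fire.
; The construction script assigns meshes and materials, plus a physical material override on the tracks.
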(event `self.ReceiveBeginPlay`
  (`TankAimingComponent.Initialise` (`self.TankAiming`) (`self.Barrel`) (`self.Turret`))
  (`TankMovementComponent.Initialise` (`self.TankMovement`) (`self.Left Track`) (`self.Right Track`)))

(event `InputAxis|AimAzimuth`
  (params (AxisValue :type "Float (single-precision)"))
  ;[1 1 1] Camera Input Binding
  (`SceneComponent.K2_AddLocalRotation` (`self.Azimuth Gimbal`) (`KismetMathLibrary.MakeRotator` 0.0 0.0 (* AxisValue (`GameplayStatics.GetWorldDeltaSeconds`) 100.0)) false false))

(event `InputAxis|MoveForward`
  (params (AxisValue :type "Float (single-precision)"))
  ;[1 1 1] Movement Component
  (`TankMovementComponent.IntendMoveForward` (`self.TankMovement`) AxisValue))

(event `InputAxis|AimElevation`
  (params (AxisValue :type "Float (single-precision)"))
  ;[1 1 1] Camera Input Binding
  (`SceneComponent.K2_AddLocalRotation` (`self.SpringArm`) (`KismetMathLibrary.MakeRotator` 0.0 (* AxisValue (`GameplayStatics.GetWorldDeltaSeconds`) 100.0)) false false))

(event `InputAxis|TurnRight`
  (params (AxisValue :type "Float (single-precision)"))
  ;[1 1 1] Movement Component
  (`TankMovementComponent.IntendTurnRight` (`self.TankMovement`) AxisValue))

(event `InputAxis|MoveBackward`
  (params (AxisValue :type "Float (single-precision)"))
  ;[1 1 1] Movement Component
  (`TankMovementComponent.IntendMoveForward` (`self.TankMovement`) AxisValue))

(event `InputAxis|TurnLeft`
  (params (AxisValue :type "Float (single-precision)"))
  ;[1 1 1] Movement Component
  (`TankMovementComponent.IntendTurnRight` (`self.TankMovement`) AxisValue))

(event `InputAction|Fire`
  (params (Key :type "Key Structure"))
  ;[1 1 1] Firing Function
  (:`Pressed`
    (`self.Fire`)))

(fn `UserConstructionScript`
  (bind _barrel (`self.Barrel`))
  (bind _turret (`self.Turret`))
  (`KismetSystemLibrary.PrintString` "Donkey : Tank_BP BeginPlay" true true (struct :`R` 1.0 :`G` 0.554582 :`A` 1.0))
  (`StaticMeshComponent.SetStaticMesh` _turret "/Game/Tank/TankParts/tank_fbx_Turret_turret_001.tank_fbx_Turret_turret_001")
  (`PrimitiveComponent.SetMaterial` _turret 0 "/Game/StarterContent/Materials/M_Metal_Gold.M_Metal_Gold")
  (`StaticMeshComponent.SetStaticMesh` _barrel "/Game/Tank/TankParts/tank_fbx_Barrel.tank_fbx_Barrel")
  (`PrimitiveComponent.SetMaterial` _barrel 0 "/Game/StarterContent/Materials/M_Wood_Oak.M_Wood_Oak")
  (`StaticMeshComponent.SetStaticMesh` (`self.Left Track`) "/Game/Tank/TankParts/tank_fbx_Track_track_001.tank_fbx_Track_track_001")
  (`PrimitiveComponent.SetMaterial` (`self.Left Track`) 0 "/Game/StarterContent/Materials/M_Wood_Oak.M_Wood_Oak")
  (`StaticMeshComponent.SetStaticMesh` (`self.Right Track`) "/Game/Tank/TankParts/tank_fbx_Track_track_001.tank_fbx_Track_track_001")
  (`PrimitiveComponent.SetMaterial` (`self.Right Track`) 0 "/Game/StarterContent/Materials/M_Wood_Oak.M_Wood_Oak")
  (`PrimitiveComponent.SetPhysMaterialOverride` (`self.Left Track`) "/Game/Tank/Track.Track")
  (`PrimitiveComponent.SetPhysMaterialOverride` (`self.Right Track`) "/Game/Tank/Track.Track"))
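; Mortar actor Blueprint built from body, dome and barrel meshes, with a TankAiming component for aiming.
; The construction script assigns the three static meshes, gives each an oak wood material, and sets Projectile_BP as the aiming component's projectile class.
; On BeginPlay it initialises TankAiming with the barrel and the dome, so the dome serves as the turret.
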(event `self.ReceiveBeginPlay`
  (`TankAimingComponent.Initialise` (`self.TankAiming`) (`self.Barrel`) (`self.Dome`)))

(fn `UserConstructionScript`
  (bind _body (`self.Body`))
  (bind _dome (`self.Dome`))
  (bind _barrel (`self.Barrel`))
  (`StaticMeshComponent.SetStaticMesh` _body "/Game/Mortar/mortar_body.mortar_body")
  (`StaticMeshComponent.SetStaticMesh` _dome "/Game/Mortar/mortar_dome.mortar_dome")
  (`StaticMeshComponent.SetStaticMesh` _barrel "/Game/Mortar/mortar_barrel.mortar_barrel")
  (`PrimitiveComponent.SetMaterial` _body 0 "/Game/BattleGrounds_sharedassets/M_Wood_Oak.M_Wood_Oak")
  (`PrimitiveComponent.SetMaterial` _dome 0 "/Game/BattleGrounds_sharedassets/M_Wood_Oak.M_Wood_Oak")
  (`PrimitiveComponent.SetMaterial` _barrel 0 "/Game/BattleGrounds_sharedassets/M_Wood_Oak.M_Wood_Oak")
  (set `TankAimingComponent.ProjectileBlueprint` "/Game/Tank/Projectile_BP.Projectile_BP_C" (`self.TankAiming`)))